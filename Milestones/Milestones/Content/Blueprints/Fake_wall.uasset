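; Fake wall actor that becomes passable once the X-ray collection event fires.
; On BeginPlay it binds to the CustomGameMode OnCollectedXray delegate, deactivates its particles and enables collision on its static mesh.
; When the delegate fires it activates the particles, turns off mesh collision and prints a debug message.
; Material swaps between solid and translucent hex materials are present but unconnected, so they never run.
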(event Custom|XrayCollected
  (Components|Activation|Activate (Variables|Default|Getparticles) false)
  (Collision|SetCollisionEnabled (Variables|Debug|GetStaticMeshComponent) "NoCollision")
  (Development|PrintString "delegate received"))

(event EventBeginPlay
  (EventDispatchers|BindEventtoOnCollectedXray (.AsCustom%20Game%20Mode (Utilities|Casting|CastToCustomGameMode (Game|GetGameMode))) (delegate Custom|XrayCollected))
  (Components|Activation|Deactivate (Variables|Default|Getparticles))
  (Collision|SetCollisionEnabled (Variables|Debug|GetStaticMeshComponent) "QueryAndPhysics"))

(event Collision|EventActorBeginOverlap
  (params (OtherActor :type Actor%20Object%20Reference)))

(event EventTick
  (params (DeltaSeconds :type Float%20%28single-precision%29)))

(fn ConstructionScript)