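; Narrow fake interior wall that turns passable on a custom collision channel once the player collects the X-ray pickup.
; It binds to the BitwiseGameMode X-ray and reset delegates at BeginPlay, starting as a blocking wall with particles and light off.
; Collection swaps in the X-ray material, shows the effects and ignores that channel; reset restores the hex material and initial state.
; The construction script passes the mesh to a WallColorChanger.
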(event Custom|XrayCollected
  ;[1 1 1] enable all the new stuff when the delegate gets activated
  (Rendering|Material|SetMaterial (Variables|Debug|GetStaticMeshComponent) 0 (Variables|Default|GetxrayActiveMaterial))
  (Components|Activation|Activate (Variables|Default|Getparticles) false)
  (Collision|SetCollisionResponsetoChannel (Variables|Debug|GetStaticMeshComponent) "ECC_GameTraceChannel2" "ECR_Ignore")
  (Rendering|SetVisibility (Variables|Default|GetPointLight) true false))

(event Custom|ResetWall
  ;[1 1 1] Initialize the actor - set values to no collison and no particles
  (Rendering|Material|SetMaterial (Variables|Debug|GetStaticMeshComponent) 0 "/Game/Visual/materials/hex_instances/M_Hex_Parent.M_Hex_Parent")
  (Components|Activation|Deactivate (Variables|Default|Getparticles))
  (Collision|SetCollisionResponsetoChannel (Variables|Debug|GetStaticMeshComponent) "ECC_GameTraceChannel2" "ECR_Block")
  (Rendering|SetVisibility (Variables|Default|GetPointLight) false false))

(event EventBeginPlay
  (bind _returnvalue (Game|GetGameMode))
  (bind _staticmeshcomponent (Variables|Debug|GetStaticMeshComponent))
  (bind _asbitwise_game_mode (Utilities|Casting|CastToBitwiseGameMode _returnvalue))
  (|CallParentFunction)
  (EventDispatchers|BindEventtoDonReset _asbitwise_game_mode (delegate Custom|ResetWall))
  (EventDispatchers|BindEventtoOnCollectedXray _asbitwise_game_mode (delegate Custom|XrayCollected))
  (Collision|SetCollisionEnabled _staticmeshcomponent "QueryAndPhysics")
  ;[1 1 1] Initialize the actor - set values to no collison and no particles
  (Components|Activation|Deactivate (Variables|Default|Getparticles))
  (Collision|SetCollisionResponsetoChannel _staticmeshcomponent "ECC_GameTraceChannel2" "ECR_Block")
  (Rendering|SetVisibility (Variables|Default|GetPointLight) false false))

(event Collision|EventActorBeginOverlap
  (params (OtherActor :type Actor%20Object%20Reference)))

(event EventTick
  (params (DeltaSeconds :type Float%20%28single-precision%29)))

(fn ConstructionScript
  (Variables|/Game/Blueprints/LevelGeometry/WallColorChanger.WallColorChanger_C|SetStatic%20Mesh (Variables|Default|GetWallColorChanger) (Variables|Debug|GetStaticMeshComponent)))

(fn NewFunction)