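; WideFakeWall is a level geometry actor that looks and blocks like a wall until the X-ray pickup is collected.
; It binds to BitwiseGameMode's X-ray collected and reset delegates on BeginPlay.
; Collection swaps the mesh material, disables collision, and turns on particles and a point light.
; Reset restores the material and shares BeginPlay's initialization, which re-enables collision and switches both effects off.
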(event Custom|XrayCollected
  ;[1 1 1] enable all the new stuff when the delegate gets activated
  (Rendering|Material|SetMaterial (Variables|Debug|GetStaticMeshComponent) 0 "/Game/Visual/materials/mi_hexInf_wide.mi_hexInf_wide")
  (Components|Activation|Activate (Variables|Default|Getparticles) false)
  (Collision|SetCollisionEnabled (Variables|Debug|GetStaticMeshComponent) "NoCollision")
  (Rendering|SetVisibility (Variables|Default|GetPointLight) true false))

(event Custom|ResetWall
  ;[1 1 1] Initialize the actor - set values to no collison and no particles
  (Rendering|Material|SetMaterial (Variables|Debug|GetStaticMeshComponent) 0 "/Game/Visual/materials/M_hex_scaled_p.M_hex_scaled_p")
  (Components|Activation|Deactivate (Variables|Default|Getparticles))
  (Collision|SetCollisionEnabled (Variables|Debug|GetStaticMeshComponent) "QueryAndPhysics")
  (Rendering|SetVisibility (Variables|Default|GetPointLight) false false))

(event EventBeginPlay
  (bind _returnvalue (Game|GetGameMode))
  (bind _asbitwise_game_mode (Utilities|Casting|CastToBitwiseGameMode _returnvalue))
  (EventDispatchers|BindEventtoDonReset _asbitwise_game_mode (delegate Custom|ResetWall))
  (EventDispatchers|BindEventtoOnCollectedXray _asbitwise_game_mode (delegate Custom|XrayCollected))
  ;[1 1 1] Initialize the actor - set values to no collison and no particles
  (Components|Activation|Deactivate (Variables|Default|Getparticles))
  (Collision|SetCollisionEnabled (Variables|Debug|GetStaticMeshComponent) "QueryAndPhysics")
  (Rendering|SetVisibility (Variables|Default|GetPointLight) false false))

(event Collision|EventActorBeginOverlap
  (params (OtherActor :type Actor%20Object%20Reference)))

(event EventTick
  (params (DeltaSeconds :type Float%20%28single-precision%29)))

(fn ConstructionScript)