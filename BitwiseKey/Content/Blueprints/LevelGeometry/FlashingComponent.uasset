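; FlashingComponent flashes material instances by switching their EmissiveColor parameter between a flashing color and a default color.
; While CurrentlyFlashing is true, Tick accumulates time and restores the default color on every material once FlashDuration is exceeded.
; The blink uses latent Delays inside a per-Tick loop, so materials are not sequenced individually, and a debug "Hello" prints each iteration.
; This graph never sets CurrentlyFlashing, fills Materials or resets the timer.
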(event EventBeginPlay)

(event EventTick
  (params (DeltaSeconds :type Float%20%28single-precision%29))
  (if (Variables|Flashing|GetCurrentlyFlashing)
    (Variables|Flashing|SetSecondsFlashing (+ DeltaSeconds (Variables|Flashing|GetSecondsFlashing)))
    (if (> (Variables|Flashing|GetSecondsFlashing) (Variables|Flashing|GetFlashDuration))
      (for _array_element (Variables|Flashing|GetMaterials)
        (Rendering|Material|SetVectorParameterValue _array_element "EmissiveColor" (Variables|Flashing|GetDefaultColor) :!class /Script/Engine.MaterialInstanceDynamic))
      (else
        (for _array_element_2 (Variables|Flashing|GetMaterials)
          (Development|PrintString "Hello")
          (Rendering|Material|SetVectorParameterValue _array_element_2 "EmissiveColor" (Variables|Flashing|GetFlashingColor) :!class /Script/Engine.MaterialInstanceDynamic)
          (Utilities|FlowControl|Delay 0.5)
          (Rendering|Material|SetVectorParameterValue _array_element_2 "EmissiveColor" (Variables|Flashing|GetDefaultColor) :!class /Script/Engine.MaterialInstanceDynamic)
          (Utilities|FlowControl|Delay 0.5))))))