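; Level geometry Blueprint that recolors a wall to match the powerup assigned to its linked SpawnPoint.
; On BeginPlay it creates a dynamic material instance for the StaticMesh and binds SetColor to the spawn point's powerup-assigned delegate if that reference is valid.
; SetColor writes the powerup color into the material's StartColor parameter.
; RebindDelegate repeats the binding for cases where SpawnPoint is not set at BeginPlay, such as randomized spawning.
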(event Custom|SetColor
  (params (PowerupColor :type Linear%20Color%20Structure))
  ;[1 1 1] next step: retrieve dynamic material instance
  (Rendering|Material|SetVectorParameterValue (Variables|Default|GetDynamic%20Material) "StartColor" PowerupColor :!class /Script/Engine.MaterialInstanceDynamic))

(event Custom|Rebind%20Delegate
  ;[1 1 1] only happens when parent is directly in level (not spawned with randomization)
  (EventDispatchers|BindEventtoDonPowUpAssignedDelegate (Variables|Default|Getspawn%20Point) (delegate Custom|SetColor)))

(event EventBeginPlay
  (bind _spawn_point (Variables|Default|Getspawn%20Point))
  (bind _returnvalue (Rendering|Material|CreateDynamicMaterialInstance (Rendering|Material|GetMaterial (Variables|Default|GetStatic%20Mesh) 0) "None" "None" :!class /Script/Engine.KismetMaterialLibrary))
  (bind _output_get (Variables|Default|SetDynamic%20Material _returnvalue))
  (Rendering|Material|SetMaterial (Variables|Default|GetStatic%20Mesh) 0 _output_get)
  ;[1 1 1] only happens when parent is directly in level (not spawned with randomization)
  (if (Utilities|IsValid _spawn_point)
    (EventDispatchers|BindEventtoDonPowUpAssignedDelegate _spawn_point (delegate Custom|SetColor))))

(event EventTick
  (params (DeltaSeconds :type Float%20%28single-precision%29)))