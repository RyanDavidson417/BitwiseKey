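; First-person player character Blueprint for the Bitwise game, handling death, pause, invisibility feedback and movement audio.
; BeginPlay creates the death and pause widgets, a MetaSound movement component and a dynamic post-process material, and binds FOV and game-mode reset delegates.
; Timelines drive FOV changes, the invisibility ripple and a death camera roll that reset cancels.
; "KillPlayer"-tagged overlaps trigger death; stamina and invisibility deactivation flash HUD bars.
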(event Custom|Decrease%20FOV%20event
  (params (TargetFov :type Integer))
  (Variables|Default|SetStartingFOV (Variables|/Script/Engine.CameraComponent|GetFieldOfView (Variables|Default|GetFirstPersonCameraComponent)))
  (bind _fov_adjustmentcurve (Timeline|Timeline_0 PlayFromStart)
    (:Update
      (Camera|SetFieldOfView (Variables|Default|GetFirstPersonCameraComponent) (Math|Float|Lerp (Variables|Default|GetStartingFOV) (Math|Conversions|ToFloat(Integer) TargetFov) _fov_adjustmentcurve)))))

(event Custom|KillPlayer
  (bind _firstpersoncameracomponent (Variables|Default|GetFirstPersonCameraComponent))
  (bind _firstpersoncameracomponent_2 (Variables|Default|GetFirstPersonCameraComponent))
  (bind _deathscreenwidget (Variables|Default|GetDeathScreenWIdget))
  (bind _deathscreenwidget_2 (Variables|Default|GetDeathScreenWIdget))
  (bind _relativerotation (Variables|/Script/Engine.SceneComponent|GetRelativeRotation _firstpersoncameracomponent_2))
  (if (not (Variables|Default|GetisDying))
    (Class|BitwiseGameMode|StopGameTimerandMusic (.AsBitwise%20Game%20Mode (Utilities|Casting|CastToBitwiseGameMode (Game|GetGameMode))))
    (Audio|PlaySound2D (Variables|Default|GetDeathAudio) 1.0 1.0 0.0 0 0)
    (CallFunction|StopPlayerInput)
    (UserInterface|Viewport|AddtoViewport _deathscreenwidget 0)
    (Variables|Default|SetCurrentWidget _deathscreenwidget_2)
    (Widget|SetVisibility _deathscreenwidget_2 "Visible")
    ;[1 1 1] death anim
    (UserInterface|Animation|PlayAnimation _deathscreenwidget (Variables|/Game/UI/ResetWidget.ResetWidget_C|GetBackgroundAnim _deathscreenwidget_2) 0.0 1 "Forward" 1.0 false)
    (Variables|/Script/Engine.CameraComponent|SetbUsePawnControlRotation _firstpersoncameracomponent_2 false)
    (Variables|Default|SetCurrentQuat _relativerotation)
    (Variables|Default|SetisDying true)
    (Variables|Default|SetTargetQuat (Math|Rotator|MakeRotator (+ (.Roll (Math|Rotator|BreakRotator _relativerotation)) 9e+01) 0.0 0.0))
    (bind _newtrack_0 (Timeline|RotationTimeline PlayFromStart)
      (:Update
        (Transformation|SetRelativeRotation _firstpersoncameracomponent (Math|Rotator|Lerp(Rotator) (Variables|Default|GetCurrentQuat) (Variables|Default|GetTargetQuat) _newtrack_0) false false)
        (if (not (Variables|Default|GetisDying))
          (Audio|Components|Audio|Stop (Variables|Default|GetRotationTimeline))
          (Transformation|SetRelativeRotation _firstpersoncameracomponent "0, 0, 0" false false :!label _label)
          (Variables|/Script/Engine.CameraComponent|SetbUsePawnControlRotation _firstpersoncameracomponent true)))
      (:Finished
        (goto _label)))))

(event Custom|ResetEvent
  (Audio|PlaySound2D "/Game/Audio/UI/Player_Reset_Bitwise_sfx_v1.Player_Reset_Bitwise_sfx_v1" 1.0 1.0 0.0 0 0)
  (Variables|Default|SetisDying false))

(event Custom|Change%20FOV%20event
  (params (TargetFov :type Integer))
  (Variables|Default|SetStartingFOV (Variables|/Script/Engine.CameraComponent|GetFieldOfView (Variables|Default|GetFirstPersonCameraComponent)))
  (bind _fov_adjustmentcurve (Timeline|Timeline PlayFromStart)
    (:Update
      (Camera|SetFieldOfView (Variables|Default|GetFirstPersonCameraComponent) (Math|Float|Lerp (Variables|Default|GetStartingFOV) (Math|Conversions|ToFloat(Integer) TargetFov) _fov_adjustmentcurve)))))

(event Custom|SetInverts
  (bind _optionssavegame (Variables|Default|GetOptionsSaveGame))
  (Variables|Default|SetbInvertXAxis (Variables|/Script/BitwiseKey.OptionsSaveGame|GetbInvertXAxis _optionssavegame))
  (Variables|Default|SetbInvertYAxis (Variables|/Script/BitwiseKey.OptionsSaveGame|GetbInvertYAxis _optionssavegame))
  (Development|PrintString "inverted"))

(event Custom|CallDeactivate
  (bind _returnvalue (Rendering|Material|GetScalarParameterValue (Variables|Default|GetRippleEffectMaterial) "active" :!class /Script/Engine.MaterialInstanceDynamic))
  (if (or (Audio|Components|Audio|IsPlaying (Variables|Default|GetInvisHumAudio)) (> _returnvalue 0.0))
    (Audio|Components|Audio|Stop (Variables|Default|GetInvisHumAudio))
    (Rendering|Material|SetScalarParameterValue (Variables|Default|GetRippleEffectMaterial) "active" 0.0 :!class /Script/Engine.MaterialInstanceDynamic)))

(event Input|EnhancedActionEvents|EnhancedInputActionIA_Pause
  (params (ActionValue :type Boolean) (ElapsedSeconds :type Float%20%28double-precision%29) (TriggeredSeconds :type Float%20%28double-precision%29) (InputAction :type Input%20Action%20Object%20Reference :default "/Game/UserInput/IA_Pause.IA_Pause"))
  (:Started
    (CallFunction|StopPlayerInput)
    (if (Utilities|IsValid (Variables|Default|GetCurrentWidget))
      (Class|BWKUserWidget|OnStartButtonPressed (Variables|Default|GetCurrentWidget))
      (Variables|Default|SetCurrentWidget 0)
      (else
        (Default|TogglePause (Variables|Default|GetPauseMenuReference))))))

(event EventBeginPlay
  (bind _returnvalue (Rendering|Material|CreateDynamicMaterialInstance "/Game/Visual/PostProcessing/PP_Invisiblity.PP_Invisiblity" "None" "None" :!class /Script/Engine.KismetMaterialLibrary))
  (Variables|Default|SetRippleEffectMaterial _returnvalue)
  (Rendering|AddorUpdateBlendable (Variables|Default|GetFirstPersonCameraComponent) _returnvalue 1.0 :!class /Script/Engine.CameraComponent)
  (Rendering|Material|SetScalarParameterValue (Variables|Default|GetRippleEffectMaterial) "active" 0.0 :!class /Script/Engine.MaterialInstanceDynamic)
  (EventDispatchers|BindEventtoDonReset (.AsBitwise%20Game%20Mode (Utilities|Casting|CastToBitwiseGameMode (Game|GetGameMode))) (delegate Custom|ResetEvent))
  (EventDispatchers|BindEventtoFonFOVIncreaseDelegate (delegate Custom|Change%20FOV%20event))
  (EventDispatchers|BindEventtoDonReset (.AsBitwise%20Game%20Mode (Utilities|Casting|CastToBitwiseGameMode (Game|GetGameMode))) (delegate Custom|CallDeactivate))
  (EventDispatchers|BindEventtoFonFOVDecreaseDelegate (delegate Custom|Decrease%20FOV%20event))
  (bind _returnvalue_2 (AddComponent|AddAudioComponent false))
  (Audio|Components|Audio|SetSound _returnvalue_2 "/Game/Audio/PlayerSounds/Movement/MS_PlayerMovement.MS_PlayerMovement")
  (Variables|Default|SetMetaMovementSound _returnvalue_2)
  (bind _returnvalue_3 (UserInterface|CreateWidget "/Game/UI/ResetWidget.ResetWidget_C"))
  (bind _output_get (Variables|Default|SetDeathScreenWIdget _returnvalue_3))
  (Class|BWKUserWidget|HideMenu _output_get)
  (bind _returnvalue_4 (UserInterface|CreateWidget "/Game/UI/PauseMenuWidget.PauseMenuWidget_C"))
  (bind _output_get_2 (Variables|Default|SetPauseMenuReference _returnvalue_4))
  (Widget|SetVisibility _output_get_2 "Hidden"))

(event Collision|EventActorBeginOverlap
  (params (OtherActor :type Actor%20Object%20Reference))
  (if (Actor|ActorHasTag OtherActor "KillPlayer")
    (CallFunction|KillPlayer)))

(event EventTick
  (params (DeltaSeconds :type Float%20%28single-precision%29)))

(event EventDisplayInteractPrompt)

(event EventActivateInvisibilityVFX
  (Audio|PlaySound2D (Variables|Default|GetSW_InvisActivate) 1.0 1.0 0.0 0 0)
  (Audio|Components|Audio|Play (Variables|Default|GetInvisHumAudio) 0.0)
  (bind _invisamount (Timeline|Timeline_1 PlayFromStart)
    (:Update
      (if (Variables|/Script/BitwiseKey.PowerupDataBase|GetbCollected (Variables|/Script/BitwiseKey.BitwiseGameState|GetInvisibilityData (.AsBitwise%20Game%20State (Utilities|Casting|CastToBitwiseGameState (Game|GetGameState)))))
        (Rendering|Material|SetScalarParameterValue (Variables|Default|GetRippleEffectMaterial) "active" _invisamount :!class /Script/Engine.MaterialInstanceDynamic)
        (else
          (CallFunction|CallDeactivate))))))

(event EventDeactivateInvisibilityVFX
  (params (bRanFullyOut :type Boolean))
  (Default|FlashInvisBar (Variables|Default|GetHUD%20Widget) bRanFullyOut)
  (Audio|PlaySound2D (Variables|Default|GetSW_InvisDeactivate) 1.0 1.0 0.0 0 0)
  (Audio|Components|Audio|Stop (Variables|Default|GetInvisHumAudio))
  (bind _deactivateripples (Timeline|Timeline_2 PlayFromStart)
    (:Update
      (Rendering|Material|SetScalarParameterValue (Variables|Default|GetRippleEffectMaterial) "active" _deactivateripples :!class /Script/Engine.MaterialInstanceDynamic))))

(event EventPlayMovementSound
  (params (IsWalking :type Integer))
  (bind _metamovementsound (Variables|Default|GetMetaMovementSound))
  (if (not (Audio|Components|Audio|IsPlaying _metamovementsound))
    (Effects|Components|ParticleSystem|SetIntParameter _metamovementsound "IsSprinting" IsWalking)
    (Class|AudioParameterControllerInterface|SetTriggerParameter _metamovementsound "Audio")
    (Audio|Components|Audio|Play _metamovementsound 0.0)))

(event EventStopMovementSound
  (bind _metamovementsound (Variables|Default|GetMetaMovementSound))
  (if (Audio|Components|Audio|IsPlaying _metamovementsound)
    (Class|AudioParameterControllerInterface|SetTriggerParameter _metamovementsound "Stop")))

(event EventDeactivateStaminaEffects
  (params (bRanFullyOut :type Boolean))
  (|CallParentFunction bRanFullyOut)
  (Development|PrintString "blueprints")
  (if (not (<= (Variables|/Script/BitwiseKey.BitwiseGameState|GetgameTimer (.AsBitwise%20Game%20State (Utilities|Casting|CastToBitwiseGameState (Game|GetGameState)))) 0.0))
    (Default|FlashStaminaBar (Variables|Default|GetHUD%20Widget) bRanFullyOut)))

(fn ConstructionScript)

(fn StopPlayerInput
  (bind _returnvalue (Game|GetPlayerController 0))
  (Input|SetInputModeGameandUI _returnvalue 0 "DoNotLock" true false)
  (Variables|/Script/Engine.PlayerController|SetbShowMouseCursor _returnvalue true))