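; Game mode for Bitwise that sets up the player's UI at startup and handles the win screen.
; BeginPlay creates the HUD, cross-links it with BP_PlayerCharacter, then adds SpSc widgets explaining Vision, Sprint, Jump and Invisibility with descriptions and, for most, controller and keyboard prompts.
; The WinGame event creates the win widget, calls its display function and hides the HUD.
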(event EventWinGame
  (bind _returnvalue (UserInterface|CreateWidget "/Game/UI/WinGame.WinGame_C"))
  (Default|DisplayWInscreen _returnvalue)
  (Variables|/Script/UMG.Widget|SetVisibility (Variables|Default|GetHUDWidget) "Hidden"))

(event EventTick
  (params (DeltaSeconds :type Float%20%28single-precision%29)))

(fn ConstructionScript)

(fn ReceiveBeginPlay
  (bind _output_get (Variables|Default|SetPlayerController (.AsPlayer%20Controller (Utilities|Casting|CastToPlayerController (Pawn|GetController (Game|GetPlayerCharacter 0))))))
  (bind _returnvalue (UserInterface|CreateWidget "/Game/UI/HUDWidget.HUDWidget_C" _output_get))
  (bind _output_get_2 (Variables|Default|SetHUDWidget _returnvalue))
  (UserInterface|Viewport|AddtoViewport _returnvalue 0)
  (bind _asbp_player_character (Utilities|Casting|CastToBP_PlayerCharacter (Game|GetPlayerCharacter 0))
    (:then
      (Variables|/Game/UI/HUDWidget.HUDWidget_C|SetPlayerCharacter (Variables|Default|GetHUDWidget) _asbp_player_character)
      (Variables|/Game/Blueprints/BP_PlayerCharacter.BP_PlayerCharacter_C|SetHUD%20Widget _asbp_player_character (Variables|Default|GetHUDWidget))
      (bind _returnvalue_2 (UserInterface|CreateWidget "/Game/UI/SplashScreens/WBP_SpSc_Vision.WBP_SpSc_Vision_C" (Variables|Default|GetPlayerController) "" "" "Fake walls and Hidden platforms will reveal themselves to you. 
Enemies will also be easier to detect"))
      (UserInterface|Viewport|AddtoViewport _returnvalue_2 0)
      (bind _returnvalue_3 (UserInterface|CreateWidget "/Game/UI/SplashScreens/WBP_SpSc_Sprint.WBP_SpSc_Sprint_C" (Variables|Default|GetPlayerController) "Press Left Joystick (L3) or either Bumper (R1 and L1) to activate Sprint" "Press [Left Shift] to activate Sprint" " 
This depletes your stamina"))
      (UserInterface|Viewport|AddtoViewport _returnvalue_3 0)
      (bind _returnvalue_4 (UserInterface|CreateWidget "/Game/UI/SplashScreens/WBP_SpSc_Jump.WBP_SpSc_Jump_C" (Variables|Default|GetPlayerController) "Press (A)" "Press [space]" " while already in the air to jump again"))
      (UserInterface|Viewport|AddtoViewport _returnvalue_4 0)
      (bind _returnvalue_5 (UserInterface|CreateWidget "/Game/UI/SplashScreens/WBP_SpSc_Invisibility.WBP_SpSc_Invisibility_C" (Variables|Default|GetPlayerController) "Press (B) to turn invisible" "Press [Q] to turn invisible" " 
This will make enemies unable to detect you - though they can still kill you if you run into them"))
      (UserInterface|Viewport|AddtoViewport _returnvalue_5 0)
      (UserInterface|Viewport|AddtoViewport _returnvalue_5 0))
    (:CastFailed
      (Development|PrintString "ERROR: player character cast failed" true true "(R=1.000000,G=0.000000,B=0.000000,A=1.000000)"))))