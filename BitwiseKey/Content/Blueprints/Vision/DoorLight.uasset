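; DoorLight is a door light Blueprint that registers its SpotLight with a BWKXROBase member, apparently for an X-ray vision effect.
; The construction script fills that member's ActorArray with the SpotLight and prints each entry's name.
; BeginPlay prints the array's size and item names as debug output.
; The ActivateXRay and DOnResetEvent calls are unwired, so this Blueprint never triggers the effect itself.
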(event EventBeginPlay
  (bind _bwk_xrobase (Variables|Default|GetBWK_XROBase))
  (bind _actorarray (Variables|/Game/Blueprints/Vision/BWK_XROBase.BWK_XROBase_C|GetActorArray _bwk_xrobase))
  (Development|PrintString (Utilities|String|Append (Utilities|String|ToString(Integer) (Utilities|Array|Length _actorarray)) "array size"))
  (for _array_element _actorarray
    (Development|PrintString (Utilities|String|Append (Utilities|GetObjectName _array_element) "array items"))))

(event Collision|EventActorBeginOverlap
  (params (OtherActor :type Actor%20Object%20Reference)))

(event EventTick
  (params (DeltaSeconds :type Float%20%28single-precision%29)))

(fn ConstructionScript
  (bind _output_get (Variables|/Game/Blueprints/Vision/BWK_XROBase.BWK_XROBase_C|SetActorArray (Variables|Default|GetBWK_XROBase) (Utilities|Array|MakeArray (Variables|Default|GetSpotLight))))
  (for _array_element _output_get
    (Development|PrintString (Utilities|String|Append (Utilities|GetObjectName _array_element) "array items"))))