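; BP_XrayLight is a light actor that switches on when the player collects the X-ray pickup.
; On BeginPlay it binds to the custom game mode's reset and X-ray collected delegates.
; Reset hides both the point light and spot light, while collection shows only the point light.
; The node that would show the spot light is disconnected, so nothing here turns it back on.
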(event Custom|XrayCollected
  ;[1 1 1] enable all the new stuff when the delegate gets activated
  (Rendering|SetVisibility (Variables|Default|GetPointLight) true false))

(event Custom|Reset
  ;[1 1 1] Initialize the actor - hide lights
  (Rendering|SetVisibility (Variables|Default|GetPointLight) false false)
  (Rendering|SetVisibility (Variables|Default|GetSpotLight) false false))

(event EventBeginPlay
  (bind _returnvalue (Game|GetGameMode))
  (bind _ascustom_game_mode (Utilities|Casting|CastToCustomGameMode _returnvalue))
  (|CallParentFunction)
  (EventDispatchers|BindEventtoDonReset _ascustom_game_mode (delegate Custom|Reset))
  (EventDispatchers|BindEventtoOnCollectedXray _ascustom_game_mode (delegate Custom|XrayCollected)))

(event Collision|EventActorBeginOverlap
  (params (OtherActor :type Actor%20Object%20Reference))
  (|CallParentFunction OtherActor) ; This node is disabled and will not be called.\nDrag off pins to build functionality.
)

(event EventTick
  (params (DeltaSeconds :type Float%20%28single-precision%29))
  (|CallParentFunction DeltaSeconds) ; This node is disabled and will not be called.\nDrag off pins to build functionality.
)

(fn ConstructionScript
  (|CallParentFunction))