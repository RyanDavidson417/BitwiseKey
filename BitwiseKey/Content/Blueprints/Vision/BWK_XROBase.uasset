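; Base Blueprint for X-ray vision objects, reacting to the player collecting an X-ray and to game resets.
; On BeginPlay it binds to the reset and X-ray-collected dispatchers on BitwiseGameMode.
; A reset deactivates every element in ActorArray.
; Collection calls ActivateXRay, which is an empty stub here.
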(event Custom|D_OnReset_Event
  (Class|TypedElementListLibrary|Reset))

(event Custom|OnCollectedXray_Event
  (CallFunction|ActivateXRay))

(event EventBeginPlay
  (bind _returnvalue (Game|GetGameMode))
  (bind _asbitwise_game_mode (Utilities|Casting|CastToBitwiseGameMode _returnvalue))
  (EventDispatchers|AssignDonReset _asbitwise_game_mode (delegate Custom|D_OnReset_Event))
  (EventDispatchers|AssignOnCollectedXray _asbitwise_game_mode (delegate Custom|OnCollectedXray_Event)))

(event EventTick
  (params (DeltaSeconds :type Float%20%28single-precision%29)))

(fn Reset
  (for _array_element (Variables|xray|GetActorArray)
    (Components|Activation|Deactivate _array_element)))

(fn ActivateXRay)