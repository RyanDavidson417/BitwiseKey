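; Base randomizer Blueprint that links placed actors to a powerup spawn so they can change color.
; When OnItemsPlaced fires, it loops over PlacedActors and looks for a WallColorChanger component on each.
; If PowerupSpawn is valid, it sets that component's SpawnPoint to it and calls RebindDelegate.
; The placement logic is not in this graph, and the warning print for actors lacking the component is unconnected.
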(event EventBeginPlay)

(event Collision|EventActorBeginOverlap
  (params (OtherActor :type Actor%20Object%20Reference)))

(event EventTick
  (params (DeltaSeconds :type Float%20%28single-precision%29)))

(event EventOnItemsPlaced
  (for _array_element (Variables|Default|GetPlacedActors)
    (if (Utilities|IsValid (Actor|GetComponentbyClass _array_element "/Game/Blueprints/LevelGeometry/WallColorChanger.WallColorChanger_C"))
      (if (Utilities|IsValid (Variables|Default|GetPowerup%20Spawn))
        (Variables|/Game/Blueprints/LevelGeometry/WallColorChanger.WallColorChanger_C|Setspawn%20Point (Actor|GetComponentbyClass _array_element "/Game/Blueprints/LevelGeometry/WallColorChanger.WallColorChanger_C") (Variables|Default|GetPowerup%20Spawn))
        (Default|RebindDelegate (Actor|GetComponentbyClass _array_element "/Game/Blueprints/LevelGeometry/WallColorChanger.WallColorChanger_C"))))))

(fn ConstructionScript)