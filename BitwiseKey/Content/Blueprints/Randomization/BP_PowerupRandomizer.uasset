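; Powerup randomizer Blueprint that notifies spawn points which powerup color they received once items are placed.
; BeginPlay runs the parent logic, then calls ReceiveOnItemsPlaced.
; OnItemsPlaced calls the parent, then loops over PlacedActors, using each actor's PowerupCollectibleBase component to fire its SpawnPoint's power-up-assigned delegate with PowerupColor.
; Tick and overlap events are disabled, and a leftover cast debug print never runs.
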(event EventBeginPlay
  (|CallParentFunction)
  (Class|BWKRandomizerBase|ReceiveonItemsPlaced))

(event Collision|EventActorBeginOverlap
  (params (OtherActor :type Actor%20Object%20Reference))
  (|CallParentFunction OtherActor) ; This node is disabled and will not be called.\nDrag off pins to build functionality.
)

(event EventTick
  (params (DeltaSeconds :type Float%20%28single-precision%29))
  (|CallParentFunction DeltaSeconds) ; This node is disabled and will not be called.\nDrag off pins to build functionality.
)

(event EventOnItemsPlaced
  (|CallParentFunction)
  (for _array_element (Variables|Default|GetPlacedActors)
    (Default|CallDonPowUpAssignedDelegate (Variables|/Script/BitwiseKey.PowerupCollectibleBase|GetSpawnPoint (Actor|GetComponentbyClass _array_element "/Script/BitwiseKey.PowerupCollectibleBase")) (Variables|/Script/BitwiseKey.PowerupCollectibleBase|GetPowerupColor (Actor|GetComponentbyClass _array_element "/Script/BitwiseKey.PowerupCollectibleBase")))))

(fn ConstructionScript
  (|CallParentFunction))