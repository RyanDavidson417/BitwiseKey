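; Randomized platform actor that stays hidden and non-solid until the player collects the X-ray pickup.
; It binds to BitwiseGameMode's reset and X-ray-collected delegates on BeginPlay.
; Collection swaps in the hex-infected material, activates the PlatformWallSystem particles, and enables visibility, collision and blocking on a custom trace channel.
; Reset restores the tech-panel material and returns it to the hidden, non-colliding start state.
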(event Custom|XrayCollected
  (bind _staticmeshcomponent (Variables|Debug|GetStaticMeshComponent))
  ;[1 1 1] enable all the new stuff when the delegate gets activated
  (Rendering|Material|SetMaterial (Variables|Debug|GetStaticMeshComponent) 0 "/Game/Visual/materials/Hex_Infected_ScaledD.Hex_Infected_ScaledD")
  (Components|Activation|Activate (Variables|Default|GetPlatformWallSystem) false)
  (Collision|SetCollisionEnabled _staticmeshcomponent "QueryAndPhysics")
  (Collision|SetCollisionResponsetoChannel _staticmeshcomponent "ECC_GameTraceChannel2" "ECR_Block")
  (Rendering|SetVisibility (Variables|Debug|GetStaticMeshComponent) true true))

(event Custom|ResetWall
  (bind _staticmeshcomponent (Variables|Debug|GetStaticMeshComponent))
  ;[1 1 1] Initialize the actor - set values to no collison and no particles
  (Rendering|Material|SetMaterial (Variables|Debug|GetStaticMeshComponent) 0 "/Game/StarterContent/Materials/M_Tech_Panel.M_Tech_Panel")
  (Components|Activation|Deactivate (Variables|Default|GetPlatformWallSystem))
  (Collision|SetCollisionEnabled _staticmeshcomponent "NoCollision")
  (Collision|SetCollisionResponsetoChannel _staticmeshcomponent "ECC_GameTraceChannel2" "ECR_Ignore")
  (Rendering|SetVisibility (Variables|Debug|GetStaticMeshComponent) false true))

(event EventBeginPlay
  (bind _returnvalue (Game|GetGameMode))
  (bind _staticmeshcomponent (Variables|Debug|GetStaticMeshComponent))
  (bind _asbitwise_game_mode (Utilities|Casting|CastToBitwiseGameMode _returnvalue))
  (EventDispatchers|BindEventtoDonReset _asbitwise_game_mode (delegate Custom|ResetWall))
  (EventDispatchers|BindEventtoOnCollectedXray _asbitwise_game_mode (delegate Custom|XrayCollected))
  (Collision|SetCollisionEnabled _staticmeshcomponent "QueryAndPhysics")
  ;[1 1 1] Initialize the actor - set values to no collison and no particles
  (Components|Activation|Deactivate (Variables|Default|GetPlatformWallSystem))
  (Collision|SetCollisionEnabled _staticmeshcomponent "NoCollision")
  (Collision|SetCollisionResponsetoChannel _staticmeshcomponent "ECC_GameTraceChannel2" "ECR_Ignore")
  (Rendering|SetVisibility (Variables|Debug|GetStaticMeshComponent) false true))

(event Collision|EventActorBeginOverlap
  (params (OtherActor :type Actor%20Object%20Reference)))

(event EventTick
  (params (DeltaSeconds :type Float%20%28single-precision%29)))

(fn ConstructionScript)