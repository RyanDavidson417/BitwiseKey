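; RPF_Room2 is a room level prefab that sets up randomized item spawn locations for two groups, G1 and XRay.
; The construction script passes each group's three location child actors to SetRandLocations, which appends those that cast to RandomItemSpawner to that group's BP_BaseRandomizer.
; Both randomizers are collected in RandomizerArray.
; The event graph has no logic.
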(event EventBeginPlay)

(event Collision|EventActorBeginOverlap
  (params (OtherActor :type Actor%20Object%20Reference)))

(event EventTick
  (params (DeltaSeconds :type Float%20%28single-precision%29)))

(fn ConstructionScript
  (bind _bp_br_g1 (Variables|Default|GetBP_BR_G1))
  (bind _bp_br_xray (Variables|Default|GetBP_BR_XRay))
  (bind _childactor (Variables|/Script/Engine.ChildActorComponent|GetChildActor _bp_br_xray))
  (bind _childactor_2 (Variables|/Script/Engine.ChildActorComponent|GetChildActor _bp_br_g1))
  (bind _asbp_base_randomizer (Utilities|Casting|CastToBP_BaseRandomizer _childactor_2))
  (bind _asbp_base_randomizer_2 (Utilities|Casting|CastToBP_BaseRandomizer _childactor))
  (CallFunction|SetRandLocations (Utilities|Array|MakeArray (Variables|Default|GetRL_G1R) (Variables|Default|GetRL_G1M) (Variables|Default|GetRL_G1L)) _asbp_base_randomizer)
  (Utilities|Array|Add (Variables|Default|GetRandomizerArray) _asbp_base_randomizer)
  (CallFunction|SetRandLocations (Utilities|Array|MakeArray (Variables|Default|GetRL_GX_F) (Variables|Default|GetRL_GX_BR) (Variables|Default|GetRL_GX_BL)) _asbp_base_randomizer_2)
  (Utilities|Array|Add (Variables|Default|GetRandomizerArray) _asbp_base_randomizer_2))

(fn SetRandLocations
  (params (location%20array :type Array%20of%20Child%20Actor%20Component%20Object%20References) (Randomizer :type BP%20Base%20Randomizer%20Object%20Reference))
  (for (_array_element _array_index) location%20array
    (bind _asrandom_item_spawner (Utilities|Casting|CastToRandomItemSpawner (Variables|/Script/Engine.ChildActorComponent|GetChildActor _array_element))
      (:then
        (Utilities|Array|Add (Variables|/Script/BitwiseKey.BWK_RandomizerBase|GetSpawnerArray Randomizer) _asrandom_item_spawner)
        (Development|PrintString "reached end of loop"))
      (:CastFailed
        (Utilities|String|LogString "ERROR: cast from child component to random Location FAILED")))))