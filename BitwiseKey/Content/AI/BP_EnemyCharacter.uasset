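; BP_EnemyCharacter is an enemy character driven by a StateTree that reacts to game-wide reset and X-ray events from BitwiseGameMode.
; On BeginPlay it binds to both delegates and sets its point light to zero intensity.
; Collecting the X-ray switches the light to high intensity.
; A game reset turns the light off again and restarts the StateTree logic.
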(event Custom|XrayCollected
  ;[1 1 1] enable all the new stuff when the delegate gets activated
  (Components|Activation|Activate (Variables|Default|GetPointLight) false)
  (Rendering|Components|Light|SetIntensity (Variables|Default|GetPointLight) 1e+04))

(event Custom|ResetEnemy
  ;[1 1 1] Initialize the actor - set values to no collison and no particles
  (Rendering|Components|Light|SetIntensity (Variables|Default|GetPointLight) 0.0))

(event Custom|ResetLogic
  (bind _statetree (Variables|Default|GetStateTree))
  (AI|Logic|StopLogic _statetree "")
  (AI|Logic|StartLogic _statetree))

(event Collision|EventActorBeginOverlap
  (params (OtherActor :type Actor%20Object%20Reference)))

(event EventTick
  (params (DeltaSeconds :type Float%20%28single-precision%29)))

(event EventBeginPlay
  (bind _returnvalue (Game|GetGameMode))
  (bind _asbitwise_game_mode (Utilities|Casting|CastToBitwiseGameMode _returnvalue))
  (|CallParentFunction)
  (EventDispatchers|BindEventtoDonReset (.AsBitwise%20Game%20Mode (Utilities|Casting|CastToBitwiseGameMode (Game|GetGameMode))) (delegate Custom|ResetLogic))
  (EventDispatchers|BindEventtoDonReset _asbitwise_game_mode (delegate Custom|ResetEnemy))
  (EventDispatchers|BindEventtoOnCollectedXray _asbitwise_game_mode (delegate Custom|XrayCollected))
  ;[1 1 1] Initialize the actor - set values to no collison and no particles
  (Rendering|Components|Light|SetIntensity (Variables|Default|GetPointLight) 0.0))

(fn ConstructionScript
  (|CallParentFunction))