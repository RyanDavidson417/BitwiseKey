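; BP_EnemyCharacter2 is an enemy character whose StateTree AI restarts when the game mode signals a reset.
; On BeginPlay it runs the parent logic, then casts the game mode to CustomGameMode and binds ResetLogic to its DOnReset event.
; ResetLogic stops and restarts the StateTree and prints a debug message.
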(event Custom|ResetLogic
  (bind _statetree (Variables|Default|GetStateTree))
  (AI|Logic|StopLogic _statetree "")
  (AI|Logic|StartLogic _statetree)
  (Development|PrintString "logic restarted"))

(event EventBeginPlay
  (|CallParentFunction)
  (EventDispatchers|BindEventtoDonReset (.AsCustom%20Game%20Mode (Utilities|Casting|CastToCustomGameMode (Game|GetGameMode))) (delegate Custom|ResetLogic)))

(event Collision|EventActorBeginOverlap
  (params (OtherActor :type Actor%20Object%20Reference)))

(event EventTick
  (params (DeltaSeconds :type Float%20%28single-precision%29)))

(fn ConstructionScript
  (|CallParentFunction))